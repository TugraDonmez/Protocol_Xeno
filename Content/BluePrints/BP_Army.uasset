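; BP_Army is an AI soldier enemy that shoots the first-person player, with a rifle socketed to its mesh and a randomized walk speed.
; Fire, unless IsSafe is set, spawns a muzzle effect and line-traces toward the player, playing gunfire and dealing damage only on a hit.
; HearSound writes the heard location and a flag to the Blackboard.
; Damage briefly simulates hip physics, then destroys the soldier.
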(event `self.ReceiveBeginPlay`
  (`SceneComponent.K2_AttachToComponent` (`self.Rifle`) (`self.Mesh`) "WeaponHandler" "SnapToTarget" "SnapToTarget" "KeepRelative" true)
  (bind _asbp_player_character_fps (cast `/Game/Characters/Player/BP_PlayerCharacterFPS` (`GameplayStatics.GetPlayerPawn` 0)))
  (set `self.Player` _asbp_player_character_fps)
  (set `CharacterMovementComponent.MaxWalkSpeed` (`KismetMathLibrary.RandomFloatInRange` 50.0 199.0) (`self.CharacterMovement`)))

(event `Fire`
  (bind _player (`self.Player`))
  (bind _returnvalue (`SceneComponent.GetSocketLocation` (`self.Rifle`) "Fire"))
  (if (not (`self.isSafe`))
    (set `self.bIsFiring` true)
    (`GameplayStatics.SpawnEmitterAtLocation` "/Game/StarterContent/Particles/P_Explosion.P_Explosion" _returnvalue (struct) (0.3 0.3 0.3))
    (bind (_outhit _returnvalue_2) (`KismetSystemLibrary.LineTraceSingle` _returnvalue (`self.K2_GetActorLocation` (`self.Player`)) "TraceTypeQuery1"))
    (if _returnvalue_2
      (if (== (`.HitActor` (`GameplayStatics.BreakHitResult` _outhit)) _player)
        (`GameplayStatics.PlaySoundAtLocation` "/Game/SFX/freesound_community-realistic-gun-fire-100696.freesound_community-realistic-gun-fire-100696" _returnvalue (struct) 1.0 1.0 0.0 null null null null)
        (`/Game/Characters/Player/BP_PlayerCharacterFPS.TakeDamage` _player 25.0)))))

(event `/Game/BluePrints/BPI_Hearable.HearSound`
  (params (TargetLocation :type "Vector Structure"))
  (bind _returnvalue (`AIBlueprintHelperLibrary.GetBlackboard` null))
  (`BlackboardComponent.SetValueAsBool` _returnvalue (`KismetStringLibrary.Conv_StringToName` "Hear") true)
  (`BlackboardComponent.SetValueAsVector` _returnvalue (`KismetStringLibrary.Conv_StringToName` "HearLocation") TargetLocation))

(event `/Game/BluePrints/BPI_GetDamage.Damage`
  (`KismetSystemLibrary.PrintString` "Damaged")
  (`SkeletalMeshComponent.SetBodySimulatePhysics` (`self.Mesh`) (`KismetStringLibrary.Conv_StringToName` "Hips") true)
  (`KismetSystemLibrary.Delay` 0.1)
  (`self.K2_DestroyActor`))

(fn `UserConstructionScript`)