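; Cinematic manager that runs the opening cutscene and scripted Turkish story subtitles for the Lina companion AI.
; On BeginPlay it creates the subtitle widget, locks input to UI, plays the first level sequence, then starts timed dialogue after a fixed delay.
; DialougeEvent picks follow-up conversations by DialougeNumber using hard-coded ShowSubtitle and Delay chains.
; Finished scenes can restore game input, end Lina's cinematic and send her to her next target.
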(event `self.ReceiveBeginPlay`
  (bind _returnvalue (`GameplayStatics.GetPlayerController` 0))
  (bind _returnvalue_2 (`|CreateWidget` "/Game/_UI/WBP_Subtitle.WBP_Subtitle_C"))
  (bind _output_get (set `self.SubtitleWidget` _returnvalue_2))
  (`UserWidget.AddToViewport` _output_get 10)
  (bind _outactors (`GameplayStatics.GetAllActorsOfClass` "/Game/Characters/Lina/BP_LinaAIRemastered.BP_LinaAIRemastered_C"))
  (set `self.LinaRef` (`|GetArrayItem` _outactors))
  (`WidgetBlueprintLibrary.SetInputMode_UIOnlyEx` _returnvalue null)
  (set `PlayerController.bShowMouseCursor` false _returnvalue)
  (bind _outactors_2 (`GameplayStatics.GetAllActorsOfClass` "/Script/LevelSequence.LevelSequenceActor"))
  (bind _output_get_2 (set `self.SequenceActor` (`|GetArrayItem` _outactors_2)))
  (`MovieSceneSequencePlayer.Play` (`LevelSequenceActor.SequencePlayer` _output_get_2))
  (`KismetSystemLibrary.Delay` 12.0)
  (`self.StartDialogue`))

(event `StartDialogue`
  (bind _subtitlewidget (`self.SubtitleWidget`))
  (bind _subtitlewidget_2 (`self.SubtitleWidget`))
  (`/Game/_UI/WBP_Subtitle.ShowSubtitle` _subtitlewidget_2 "\"Merhaba Dr. Arman\"")
  (`KismetSystemLibrary.Delay` 2.0)
  (`/Game/_UI/WBP_Subtitle.ShowSubtitle` _subtitlewidget_2 "\"Rahatsız ettim biliyorum ama konuşmamız lazım.\"")
  (`KismetSystemLibrary.Delay` 3.0)
  (`/Game/_UI/WBP_Subtitle.ShowSubtitle` _subtitlewidget_2 "\"Eşin Dr. Jane yakın arkadaşımdı biliyorsun.\"")
  (`KismetSystemLibrary.Delay` 2.0)
  (`/Game/_UI/WBP_Subtitle.ShowSubtitle` _subtitlewidget_2 "\"Onun sayesinde burada bir bilim insanıyım.\"")
  (`KismetSystemLibrary.Delay` 2.0)
  (`/Game/_UI/WBP_Subtitle.ShowSubtitle` _subtitlewidget_2 "\"O benim arkamı her zaman kollardı.\"")
  (`KismetSystemLibrary.Delay` 2.0)
  (`/Game/_UI/WBP_Subtitle.ShowSubtitle` _subtitlewidget_2 "\"... Bence burada bir şeyler yanlış gidiyor.\"")
  (`KismetSystemLibrary.Delay` 2.0)
  (`/Game/_UI/WBP_Subtitle.ShowSubtitle` _subtitlewidget_2 "\"Biz bir gizli proje üzerinde çalışıyorduk.\"")
  (`KismetSystemLibrary.Delay` 2.0)
  (`/Game/_UI/WBP_Subtitle.ShowSubtitle` _subtitlewidget_2 "\"Uzay Biyolojisi altında garip incelemeler yaptım.\"")
  (`KismetSystemLibrary.Delay` 2.0)
  (`/Game/_UI/WBP_Subtitle.ShowSubtitle` _subtitlewidget "\"Detaylarını bilmiyorum bana genelde ayak işi yaptırırlardı.\"")
  (`KismetSystemLibrary.Delay` 3.0)
  (`/Game/_UI/WBP_Subtitle.ShowSubtitle` _subtitlewidget "\"Dr. Jane'nin ölümünün ardından bu olayı araştırmaya başladım ve bir şeyler buldum.\"")
  (`KismetSystemLibrary.Delay` 3.0)
  (`/Game/_UI/WBP_Subtitle.ShowSubtitle` _subtitlewidget "\"Benim ofisime gelebilirmisin sana bir dosya göstermeliyim.\"")
  (`KismetSystemLibrary.Delay` 2.0)
  (`/Game/_UI/WBP_Subtitle.ShowSubtitle` _subtitlewidget "\"Masamın üzerinde duruyor\"")
  (`KismetSystemLibrary.Delay` 2.0)
  (`/Game/_UI/WBP_Subtitle.ShowSubtitle` _subtitlewidget "\"Beni takip et.\"")
  (`KismetSystemLibrary.Delay` 1.0)
  (`/Game/_UI/WBP_Subtitle.HideSubtitle` _subtitlewidget_2)
  (`self.UnlockPlayer`))

(event `UnlockPlayer`
  (`WidgetBlueprintLibrary.SetInputMode_GameOnly` (`GameplayStatics.GetPlayerController` 0))
  (`/Game/Characters/Lina/BP_LinaAIRemastered.EndCinematic` (`self.LinaRef`)))

(event `DialougeEvent`
  (bind _subtitlewidget (`self.SubtitleWidget`))
  (bind _subtitlewidget_2 (`self.SubtitleWidget`))
  (bind _subtitlewidget_3 (`self.SubtitleWidget`))
  (bind _subtitlewidget_4 (`self.SubtitleWidget`))
  (switch `int` (`self.DialougeNumber`)
    (:`Default`
      (`/Game/_UI/WBP_Subtitle.ShowSubtitle` _subtitlewidget "Hmm")
      (`KismetSystemLibrary.Delay` 2.0)
      (`/Game/_UI/WBP_Subtitle.HideSubtitle` _subtitlewidget))
    (:`0`
      (`/Game/_UI/WBP_Subtitle.ShowSubtitle` _subtitlewidget_2 "\"Evet bu dosyadan anladığım kadarıyla\"")
      (`KismetSystemLibrary.Delay` 2.0)
      (`/Game/_UI/WBP_Subtitle.ShowSubtitle` _subtitlewidget_2 "\"Bir Form bulmuşlar ve Jane onun üzerinde araştırma yapıyordu\"")
      (`KismetSystemLibrary.Delay` 3.0)
      (`/Game/_UI/WBP_Subtitle.ShowSubtitle` _subtitlewidget_2 "\"Gizli tutulması lazımmış ve bence ölümünün bu ile alakası var\"")
      (`KismetSystemLibrary.Delay` 2.0)
      (`/Game/_UI/WBP_Subtitle.ShowSubtitle` _subtitlewidget_2 "\"Diğer bahsettiği dosyayı bulamadım\"")
      (`KismetSystemLibrary.Delay` 2.0)
      (`/Game/_UI/WBP_Subtitle.ShowSubtitle` _subtitlewidget_2 "\"Arşiv'e kaldırıldığı yazılmış\"")
      (`KismetSystemLibrary.Delay` 1.0)
      (`/Game/_UI/WBP_Subtitle.ShowSubtitle` _subtitlewidget_2 "\"Odadan çıkıp Arşive gidip araştıralım.\"")
      (`KismetSystemLibrary.Delay` 2.0)
      (`/Game/_UI/WBP_Subtitle.HideSubtitle` _subtitlewidget_2)
      (`self.NewTarget`)
      (`self.UnlockPlayer`))
    (:`1`
      (`/Game/_UI/WBP_Subtitle.ShowSubtitle` _subtitlewidget_3 "\"Demek buldun. Gerçekten çok iyisin.\"")
      (`KismetSystemLibrary.Delay` 2.0)
      (`/Game/_UI/WBP_Subtitle.ShowSubtitle` _subtitlewidget_3 "\"Vay canına inanamıyorum. Çok korkutucu\"")
      (`KismetSystemLibrary.Delay` 2.0)
      (`/Game/_UI/WBP_Subtitle.ShowSubtitle` _subtitlewidget_3 "\"Demek ki Jane gerçekten birşeyler saklıyormuş.\"")
      (`KismetSystemLibrary.Delay` 2.0)
      (`/Game/_UI/WBP_Subtitle.ShowSubtitle` _subtitlewidget_3 "\"O kayalığı incelemen lazım arman.\"")
      (`KismetSystemLibrary.Delay` 2.0)
      (`/Game/_UI/WBP_Subtitle.ShowSubtitle` _subtitlewidget_3 "\"4. Bölgeye Resepsiyona çıktığın zaman sağa dönerek gidebilirsin.\"")
      (`KismetSystemLibrary.Delay` 3.0)
      (`/Game/_UI/WBP_Subtitle.ShowSubtitle` _subtitlewidget_3 "\"Ben ofisimden oradaki çalışanları Evelyn Çağırmış gibi uzaklaştıracağım.\"")
      (`KismetSystemLibrary.Delay` 3.0)
      (`/Game/_UI/WBP_Subtitle.ShowSubtitle` _subtitlewidget_3 "\"Dönünce direk yanıma gel.\"")
      (`KismetSystemLibrary.Delay` 2.0)
      (`/Game/_UI/WBP_Subtitle.HideSubtitle` _subtitlewidget_3))
    (:`2`
      (`/Game/_UI/WBP_Subtitle.ShowSubtitle` _subtitlewidget_4 "Hmm Evelyn beni neden önemsedi ki")
      (`KismetSystemLibrary.Delay` 2.0)
      (`/Game/_UI/WBP_Subtitle.HideSubtitle` _subtitlewidget_4))))

(event `NewTarget`
  (bind _linaref (`self.LinaRef`))
  (`/Game/Characters/Lina/BP_LinaAIRemastered.EndCinematic` _linaref)
  (`/Game/Characters/Lina/BP_LinaAIRemastered.SetNextTarget` _linaref))

(fn `UserConstructionScript`)