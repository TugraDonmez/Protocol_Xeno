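; BP_Generator is a generator actor that responds to an Activate event by powering up and opening a linked door.
; Activation prints a status message, swaps the light mesh to a green emissive material and turns its point light green.
; It then calls DoorOpening on the referenced door and, if the Event flag is set, spawns a BP_XenoA at the referenced Location actor's transform.
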(event `/Game/BluePrints/BPI_Activatable.Activate`
  (`KismetSystemLibrary.PrintString` "Jeneratör aktif")
  (`PrimitiveComponent.SetMaterial` (`self.Light`) 0 "/Game/StarterContent/M_E_Green.M_E_Green")
  (`LightComponent.SetLightColor` (`self.PointLight`) (struct :`G` 1.0 :`B` 0.033831 :`A` 1.0) true)
  (`/Game/QA_Office/Blueprints/BP_PanicDoor.DoorOpening` (`self.OpenedDoor`))
  (if (`self.Event`)
    (`|SpawnActorFromClass` "/Game/Characters/Alien/BP_XenoA.BP_XenoA_C" (`self.GetTransform` (`self.Location`)) "Undefined" "MultiplyWithRoot" null null)))

(fn `UserConstructionScript`)