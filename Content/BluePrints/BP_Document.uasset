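; BP_Document is a readable document actor that shows its title, body and author in a WBP_DocumentViewer widget.
; OpenDocument adds the widget to the viewport, switches player 0 to Game and UI input, blocks movement and shows the cursor.
; If a Cinematic reference is valid, it also triggers that object's dialogue event at DialougeIndex, then destroys itself.
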(event `OpenDocument`
  (bind _returnvalue (`GameplayStatics.GetPlayerController` 0))
  (bind _cinematic (`self.Cinematic`))
  (bind _returnvalue_2 (`|CreateWidget` "/Game/_UI/WBP_DocumentViewer.WBP_DocumentViewer_C"))
  (`/Game/_UI/WBP_DocumentViewer.SetDocumentData` _returnvalue_2 (`self.DocumentTitle`) (`self.DocumentBody`) (`self.AuthorName`))
  (`UserWidget.AddToViewport` _returnvalue_2 0)
  (`WidgetBlueprintLibrary.SetInputMode_GameAndUIEx` _returnvalue null "DoNotLock" false)
  (`Controller.SetIgnoreMoveInput` _returnvalue true)
  (set `PlayerController.bShowMouseCursor` true _returnvalue)
  (if (`KismetSystemLibrary.IsValid` _cinematic)
    (set `/Game/BluePrints/BP_CinematicManager1.DialougeNumber` (`self.DialougeIndex`) _cinematic)
    (`/Game/BluePrints/BP_CinematicManager1.DialougeEvent` _cinematic)
    (`self.K2_DestroyActor`)))

(fn `UserConstructionScript`)