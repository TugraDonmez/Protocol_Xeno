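; Blueprint that plays a scripted subtitle dialogue in Turkish between Arman and Dr. Marcus, who briefs the player on the facility objective.
; On BeginPlay it creates a WBP_Subtitle widget and adds it to the viewport.
; It then shows hardcoded lines through ShowSubtitle at fixed Delay intervals and hides the subtitle at the end.
; The sequence has no trigger or audio; overlap and tick events are unused.
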(event `self.ReceiveBeginPlay`
  (bind _subtitle_widget (`self.Subtitle Widget`))
  (bind _returnvalue (`|CreateWidget` "/Game/_UI/WBP_Subtitle.WBP_Subtitle_C"))
  (bind _output_get (set `self.Subtitle Widget` _returnvalue))
  (`UserWidget.AddToViewport` _output_get 0)
  (`/Game/_UI/WBP_Subtitle.ShowSubtitle` (`self.Subtitle Widget`) "\"Arman: Burası da neresi\"")
  (`KismetSystemLibrary.Delay` 2.0)
  (`/Game/_UI/WBP_Subtitle.ShowSubtitle` (`self.Subtitle Widget`) "\"Marcus: Merhaba arman, Ben Dr. Marcus\"")
  (`KismetSystemLibrary.Delay` 2.0)
  (`/Game/_UI/WBP_Subtitle.ShowSubtitle` (`self.Subtitle Widget`) "\"Marcus: Beni tanımıyorsun. Gizli bir çalışandım. Şu an tesisin mikrafonlarından konuşuyorum.\"")
  (`KismetSystemLibrary.Delay` 2.0)
  (`/Game/_UI/WBP_Subtitle.ShowSubtitle` (`self.Subtitle Widget`) "\"Marcus: Seni biliyorum, Jane senden bahsederdi.\"")
  (`KismetSystemLibrary.Delay` 2.0)
  (`/Game/_UI/WBP_Subtitle.ShowSubtitle` (`self.Subtitle Widget`) "\"Marcus: Kafanda çok soru var biliyorum.\"")
  (`KismetSystemLibrary.Delay` 2.0)
  (`/Game/_UI/WBP_Subtitle.ShowSubtitle` _subtitle_widget "\"Marcus: Odamda sıkıştım ve yanımda tüm cevapları içeren dosyalar var.\"")
  (`KismetSystemLibrary.Delay` 2.0)
  (`/Game/_UI/WBP_Subtitle.ShowSubtitle` (`self.Subtitle Widget`) "\"Marcus: Çıkış yanımda kapıyı açmak için Evelyn'in telefonu lazım \"")
  (`KismetSystemLibrary.Delay` 2.0)
  (`/Game/_UI/WBP_Subtitle.ShowSubtitle` _subtitle_widget "\"Marcus: Önce telefonu alarak kilitli odaya girmen lazım, sonra oradaki jeneratörü çalıştır ve benim yanıma gel\"")
  (`KismetSystemLibrary.Delay` 2.0)
  (`/Game/_UI/WBP_Subtitle.ShowSubtitle` (`self.Subtitle Widget`) "\"Marcus: Fakat burası çok tehlikeli herkes burada.\"")
  (`KismetSystemLibrary.Delay` 2.0)
  (`/Game/_UI/WBP_Subtitle.ShowSubtitle` (`self.Subtitle Widget`) "\"Marcus: Tasarladığım silahı kullanabildiğine göre bunu yapabilirsin.\"")
  (`KismetSystemLibrary.Delay` 2.0)
  (`/Game/_UI/WBP_Subtitle.HideSubtitle` (`self.Subtitle Widget`)))

(fn `UserConstructionScript`)