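; Sound-reactive column that switches its light from red to green when it hears a sound whose target location is close to the column.
; HearSound calls OpenEnergy, which checks the distance to ColumnMesh, then swaps the Light material, recolors the PointLight and sets the Open flag.
; After a fixed delay, HearSound calls CloseEnergy to restore red and clear Open, regardless of whether the distance check passed.
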(event `/Game/BluePrints/BPI_Hearable.HearSound`
  (params (TargetLocation :type "Vector Structure"))
  (`self.OpenEnergy` TargetLocation)
  (`KismetSystemLibrary.Delay` 5.0)
  (`self.CloseEnergy`))

(event `OpenEnergy`
  (params (TargetLocation :type "Vector Structure"))
  (if (< (`KismetMathLibrary.Vector_Distance` TargetLocation (`SceneComponent.K2_GetComponentLocation` (`self.ColumnMesh`))) 100.0)
    (`PrimitiveComponent.SetMaterial` (`self.Light`) 0 "/Game/StarterContent/M_E_Green.M_E_Green")
    (`LightComponent.SetLightColor` (`self.PointLight`) (struct :`R` 0.025116 :`G` 1.0 :`A` 1.0) true)
    (set `self.Open` true)))

(event `CloseEnergy`
  (`PrimitiveComponent.SetMaterial` (`self.Light`) 0 "/Game/StarterContent/M_E_Red.M_E_Red")
  (`LightComponent.SetLightColor` (`self.PointLight`) (struct :`R` 1.0 :`G` 0.05659 :`A` 1.0) true)
  (set `self.Open` false))

(fn `UserConstructionScript`)