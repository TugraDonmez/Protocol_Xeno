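; BP_Escape is a trigger actor that shows the escape screen when the FPS player character enters its collision volume.
; On overlap it switches to UI-only input, shows the mouse cursor and adds a WBP_Escape widget to the viewport.
; It then plays the first LevelSequenceActor found in the level on an endless loop, relying on a class search rather than a set reference.
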(event `self.CollisionComponent.OnComponentBeginOverlap`
  (params (OverlappedComponent :type "PrimitiveComponent Object Reference") (OtherActor :type "Actor Object Reference") (OtherComp :type "PrimitiveComponent Object Reference") (OtherBodyIndex :type Integer) (bFromSweep :type Boolean) (SweepResult :type "HitResult Structure (by ref)"))
  (bind _returnvalue (`GameplayStatics.GetPlayerController` 0))
  (cast `/Game/Characters/Player/BP_PlayerCharacterFPS` OtherActor)
  (`WidgetBlueprintLibrary.SetInputMode_UIOnlyEx` _returnvalue null)
  (set `PlayerController.bShowMouseCursor` true _returnvalue)
  (bind _returnvalue_2 (`|CreateWidget` "/Game/_UI/WBP_Escape.WBP_Escape_C"))
  (`UserWidget.AddToViewport` _returnvalue_2 0)
  (bind _outactors (`GameplayStatics.GetAllActorsOfClass` "/Script/LevelSequence.LevelSequenceActor"))
  (bind _output_get (set `self.Sequence Actor` (`|GetArrayItem` _outactors)))
  (`MovieSceneSequencePlayer.PlayLooping` (`LevelSequenceActor.SequencePlayer` _output_get) -1))

(fn `UserConstructionScript`)