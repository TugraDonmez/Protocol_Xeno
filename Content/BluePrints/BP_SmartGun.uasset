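; BP_SmartGun is a gun Blueprint that shows one of three weapon modes through two indicator lights.
; Events Mode_0, Mode_1 and Mode_2 swap both light meshes to green, blue or red emissive materials, without changing WeaponMode themselves.
; BeginPlay sets WeaponMode to 0 and queries all BPI_Hearable actors, though the result is unused here.
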(event `self.ReceiveBeginPlay`
  (`GameplayStatics.GetAllActorsWithInterface` "/Game/BluePrints/BPI_Hearable.BPI_Hearable_C")
  (set `self.weaponMode` 0))

(event `Mode_0`
  (`PrimitiveComponent.SetMaterial` (`self.Light`) 0 "/Game/StarterContent/M_E_Green.M_E_Green")
  (`PrimitiveComponent.SetMaterial` (`self.Light1`) 0 "/Game/StarterContent/M_E_Green.M_E_Green"))

(event `Mode_1`
  (`PrimitiveComponent.SetMaterial` (`self.Light`) 0 "/Game/StarterContent/M_E_Blue.M_E_Blue")
  (`PrimitiveComponent.SetMaterial` (`self.Light1`) 0 "/Game/StarterContent/M_E_Blue.M_E_Blue"))

(event `Mode_2`
  (`PrimitiveComponent.SetMaterial` (`self.Light`) 0 "/Game/StarterContent/M_E_Red.M_E_Red")
  (`PrimitiveComponent.SetMaterial` (`self.Light1`) 0 "/Game/StarterContent/M_E_Red.M_E_Red"))

(fn `UserConstructionScript`)