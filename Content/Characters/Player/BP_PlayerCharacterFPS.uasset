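; First-person player character with Enhanced Input movement, sprint, jump, crosshair HUD, damage handling and a restart screen.
; It attaches a three-mode SmartGun whose primary and secondary fire spend energy on traces or area effects, sending hearing, activate, damage or explode interface messages.
; An interact line trace opens documents, photos and the gun pickup or collects the key card, and can also recharge gun energy.
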(event `AddGun`
  (bind _returnvalue (`|SpawnActorFromClass` "/Game/BluePrints/BP_SmartGun.BP_SmartGun_C" (`SceneComponent.GetRelativeTransform` (`self.GunTransform`)) "Undefined" "MultiplyWithRoot" null null))
  (set `self.CurrentWeapon` _returnvalue)
  (`self.K2_AttachToComponent` _returnvalue (`self.FP_Camera`) "None" "KeepRelative" "KeepRelative" "KeepRelative" true)
  (bind _asbp_smart_gun (cast `/Game/BluePrints/BP_SmartGun` (`self.CurrentWeapon`)))
  (bind _output_get (set `/Game/BluePrints/BP_SmartGun.weaponMode` 1 _asbp_smart_gun))
  (set `self.WeaponModeControl` _output_get)
  (`/Game/BluePrints/BP_SmartGun.Mode_0` _asbp_smart_gun)
  (`KismetSystemLibrary.Delay` 0.1)
  (`Widget.SetVisibility` (`/Game/_UI/WBP_Crosshair.EnergyText` (`self.Widget`)) "Visible"))

(event `self.ReceiveBeginPlay`
  (bind _asplayer_controller (cast `PlayerController` (`self.GetController`)))
  (message `EnhancedInputSubsystemInterface.AddMappingContext` (pcsubsystem `EnhancedInputLocalPlayerSubsystem` _asplayer_controller) "/Game/Input/NewInput/Mappings/IMC_Player.IMC_Player" 0 (struct))
  (bind _returnvalue (`|CreateWidget` "/Game/_UI/WBP_Crosshair.WBP_Crosshair_C"))
  (bind _output_get (set `self.Widget` _returnvalue))
  (`/Game/_UI/WBP_Crosshair.SetEnergy` _output_get (`KismetStringLibrary.Conv_DoubleToString` (`/Game/BluePrints/BP_SmartGun.currentEnergy` (`self.CurrentWeapon`))))
  (set `Widget.Visibility` "Hidden" (`/Game/_UI/WBP_Crosshair.EnergyText` _returnvalue))
  (`UserWidget.AddToViewport` _returnvalue 0)
  (`UserWidget.AddToViewport` _output_get 0)
  (if (`KismetSystemLibrary.IsValid` (`self.CurrentWeapon`))
    (bind _outactors (`GameplayStatics.GetAllActorsOfClass` "/Game/BluePrints/BP_SmartGun.BP_SmartGun_C"))
    (add `/Game/BluePrints/BP_SmartGun.OnEnergyHit` (`|GetArrayItem` _outactors) (delegate `OnEnergyHitReceived`))))

(event `OnEnergyHitReceived`
  (params (HitActor :type "Actor Object Reference"))
  (if (`KismetSystemLibrary.DoesImplementInterface` HitActor "/Game/BluePrints/BPI_Activatable.BPI_Activatable_C")
    (message `/Game/BluePrints/BPI_Activatable.Activate` HitActor)))

(event `EnhancedInput|/Game/Input/NewInput/Action/IA_WeaponMode_1`
  (params (ActionValue :type Boolean) (ElapsedSeconds :type "Float (double-precision)") (TriggeredSeconds :type "Float (double-precision)") (InputAction :type "InputAction Object Reference" :default "/Game/Input/NewInput/Action/IA_WeaponMode_1.IA_WeaponMode_1"))
  (:`Triggered`
    (bind _asbp_smart_gun (cast `/Game/BluePrints/BP_SmartGun` (`self.CurrentWeapon`)))
    (bind _output_get (set `/Game/BluePrints/BP_SmartGun.weaponMode` 1 _asbp_smart_gun))
    (set `self.WeaponModeControl` _output_get)
    (`/Game/BluePrints/BP_SmartGun.Mode_0` _asbp_smart_gun)))

(event `EnhancedInput|/Game/Input/NewInput/Action/IA_MoveFPS`
  (params (ActionValue :type "Vector2D Structure") (ElapsedSeconds :type "Float (double-precision)") (TriggeredSeconds :type "Float (double-precision)") (InputAction :type "InputAction Object Reference" :default "/Game/Input/NewInput/Action/IA_MoveFPS.IA_MoveFPS"))
  ; Inputs
  ;; Movement
  (:`Triggered`
    (`self.AddMovementInput` (`self.GetActorForwardVector`) (`KismetMathLibrary.BreakVector2D` ActionValue))))

(event `EnhancedInput|/Game/Input/NewInput/Action/IA_MoveFPS`
  (params (ActionValue :type "Vector2D Structure") (ElapsedSeconds :type "Float (double-precision)") (TriggeredSeconds :type "Float (double-precision)") (InputAction :type "InputAction Object Reference" :default "/Game/Input/NewInput/Action/IA_MoveFPS.IA_MoveFPS"))
  ; Inputs
  ;; Movement
  (:`Triggered`
    (`self.AddMovementInput` (`self.GetActorRightVector`) (`.Y` (`KismetMathLibrary.BreakVector2D` ActionValue)))))

(event `EnhancedInput|/Game/Input/NewInput/Action/IA_WeaponMode_2`
  (params (ActionValue :type Boolean) (ElapsedSeconds :type "Float (double-precision)") (TriggeredSeconds :type "Float (double-precision)") (InputAction :type "InputAction Object Reference" :default "/Game/Input/NewInput/Action/IA_WeaponMode_2.IA_WeaponMode_2"))
  (:`Triggered`
    (bind _asbp_smart_gun (cast `/Game/BluePrints/BP_SmartGun` (`self.CurrentWeapon`)))
    (bind _output_get (set `/Game/BluePrints/BP_SmartGun.weaponMode` 2 _asbp_smart_gun))
    (set `self.WeaponModeControl` _output_get)
    (`/Game/BluePrints/BP_SmartGun.Mode_1` _asbp_smart_gun)))

(event `EnhancedInput|/Game/Input/NewInput/Action/IA_LookFPS`
  (params (ActionValue :type "Vector2D Structure") (ElapsedSeconds :type "Float (double-precision)") (TriggeredSeconds :type "Float (double-precision)") (InputAction :type "InputAction Object Reference" :default "/Game/Input/NewInput/Action/IA_LookFPS.IA_LookFPS"))
  (bind (_x _y) (`KismetMathLibrary.BreakVector2D` ActionValue))
  ; Inputs
  ;; Movement
  (:`Triggered`
    (`self.AddControllerYawInput` _x)
    (`self.AddControllerPitchInput` _y)))

(event `EnhancedInput|/Game/Input/NewInput/Action/IA_WeaponMode_3`
  (params (ActionValue :type Boolean) (ElapsedSeconds :type "Float (double-precision)") (TriggeredSeconds :type "Float (double-precision)") (InputAction :type "InputAction Object Reference" :default "/Game/Input/NewInput/Action/IA_WeaponMode_3.IA_WeaponMode_3"))
  (:`Triggered`
    (bind _asbp_smart_gun (cast `/Game/BluePrints/BP_SmartGun` (`self.CurrentWeapon`)))
    (bind _output_get (set `/Game/BluePrints/BP_SmartGun.weaponMode` 3 _asbp_smart_gun))
    (set `self.WeaponModeControl` _output_get)
    (`/Game/BluePrints/BP_SmartGun.Mode_2` _asbp_smart_gun)))

(event `EnhancedInput|/Game/Input/NewInput/Action/IA_SprintFPS`
  (params (ActionValue :type Boolean) (ElapsedSeconds :type "Float (double-precision)") (TriggeredSeconds :type "Float (double-precision)") (InputAction :type "InputAction Object Reference" :default "/Game/Input/NewInput/Action/IA_SprintFPS.IA_SprintFPS"))
  (bind _charactermovement (`self.CharacterMovement`))
  ; Inputs
  ;; Movement
  (:`Started`
    (bind _ascharacter_movement_component (cast `CharacterMovementComponent` _charactermovement))
    (set `CharacterMovementComponent.MaxWalkSpeed` 700.0 _ascharacter_movement_component))
  (:`Completed`
    (bind _ascharacter_movement_component_2 (cast `CharacterMovementComponent` _charactermovement))
    (set `CharacterMovementComponent.MaxWalkSpeed` 400.0 _ascharacter_movement_component_2)))

(event `Key|Q`
  (params (Key :type "Key Structure"))
  (:`Pressed`
    (`|ExecutionSequence`
      (:`then_0`
        (bind _foundwidgets (`WidgetBlueprintLibrary.GetAllWidgetsOfClass` "/Game/_UI/WBP_DocumentViewer.WBP_DocumentViewer_C"))
        (bind _output (`|GetArrayItem` _foundwidgets))
        (if (`KismetSystemLibrary.IsValid` _output)
          (`/Game/_UI/WBP_DocumentViewer.CloseDocument` _output)))
      (:`then_1`
        (bind _foundwidgets_2 (`WidgetBlueprintLibrary.GetAllWidgetsOfClass` "/Game/_UI/WBP_PictureViewer.WBP_PictureViewer_C"))
        (bind _output_2 (`|GetArrayItem` _foundwidgets_2))
        (if (`KismetSystemLibrary.IsValid` _output_2)
          (`/Game/_UI/WBP_PictureViewer.ClosePhoto` _output_2))))))

(event `EnhancedInput|/Game/Input/NewInput/Action/IA_Fire_Primary`
  (params (ActionValue :type Boolean) (ElapsedSeconds :type "Float (double-precision)") (TriggeredSeconds :type "Float (double-precision)") (InputAction :type "InputAction Object Reference" :default "/Game/Input/NewInput/Action/IA_Fire_Primary.IA_Fire_Primary"))
  (:`Triggered`
    (`self.Shoot_Primary`)))

(event `EnhancedInput|/Game/Input/NewInput/Action/IA_JumpFPS`
  (params (ActionValue :type Boolean) (ElapsedSeconds :type "Float (double-precision)") (TriggeredSeconds :type "Float (double-precision)") (InputAction :type "InputAction Object Reference" :default "/Game/Input/NewInput/Action/IA_JumpFPS.IA_JumpFPS"))
  ; Inputs
  ;; Movement
  (:`Started`
    (`self.Jump`))
  (:`Completed`
    (`self.StopJumping`)))

(event `EnhancedInput|/Game/Input/NewInput/Action/IA_Fire_Secondary`
  (params (ActionValue :type Boolean) (ElapsedSeconds :type "Float (double-precision)") (TriggeredSeconds :type "Float (double-precision)") (InputAction :type "InputAction Object Reference" :default "/Game/Input/NewInput/Action/IA_Fire_Secondary.IA_Fire_Secondary"))
  (:`Triggered`
    (`self.Shoot_Secondary`)))

(event `EnhancedInput|/Game/Input/NewInput/Action/IA_Interact`
  (params (ActionValue :type Boolean) (ElapsedSeconds :type "Float (double-precision)") (TriggeredSeconds :type "Float (double-precision)") (InputAction :type "InputAction Object Reference" :default "/Game/Input/NewInput/Action/IA_Interact.IA_Interact"))
  (bind _fp_camera (`self.FP_Camera`))
  (:`Triggered`
    (`KismetSystemLibrary.PrintString` "Interact")
    (`|ExecutionSequence`
      (:`then_0`
        (bind _outhit (`KismetSystemLibrary.LineTraceSingle` (`SceneComponent.K2_GetComponentLocation` (`self.FP_Camera`)) (+ (`SceneComponent.K2_GetComponentLocation` _fp_camera) (* (`SceneComponent.GetForwardVector` _fp_camera) 200)) "TraceTypeQuery1"))
        (`|ExecutionSequence`
          (:`then_0`
            (bind (_bblockinghit _binitialoverlap _time _distance _location _impactpoint _normal _impactnormal _physmat _hitactor) (`GameplayStatics.BreakHitResult` _outhit))
            (bind _asbp_document (cast `/Game/BluePrints/BP_Document` _hitactor))
            (`/Game/BluePrints/BP_Document.OpenDocument` _asbp_document))
          (:`then_1`
            (bind _asbp_photo (cast `/Game/BluePrints/BP_Photo` _hitactor))
            (`/Game/BluePrints/BP_Photo.OpenPhoto` _asbp_photo))
          (:`then_2`
            (bind _asbp_smart_gun_take (cast `/Game/BluePrints/BP_SmartGunTake` _hitactor)
              (:`then`
                (`KismetSystemLibrary.PrintString` "nonfail")
                (`/Game/BluePrints/BP_SmartGunTake.OpenWeapon` _asbp_smart_gun_take))
              (:`CastFailed`
                (`KismetSystemLibrary.PrintString` "fail"))))
          (:`then_3`
            (bind _asbp_card (cast `/Game/BluePrints/BP_Card` _hitactor))
            (set `self.haveKey` true)
            (`self.K2_DestroyActor` _asbp_card))))
      (:`then_1`
        (if (`self.ChargeT`)
          (`self.ChargeWeapon` 0.0))))))

(event `/Game/BluePrints/BPI_Interact.ChargeWeapon`
  (params (ChargeAmount :type "Float (double-precision)"))
  (bind _as_bp_smart_gun (`self.As BP Smart Gun`))
  (if (`self.CanChargeEnergy`)
    (bind _output_get (set `/Game/BluePrints/BP_SmartGun.currentEnergy` (`/Game/BluePrints/BP_SmartGun.maxEnergy` _as_bp_smart_gun) _as_bp_smart_gun))
    (`/Game/_UI/WBP_Crosshair.SetEnergy` (`self.Widget`) (`KismetStringLibrary.Conv_DoubleToString` _output_get))
    (set `self.ChargeT` false)
    (`GameplayStatics.PlaySound2D` "/Engine/VREditor/Sounds/VR_confirm.VR_confirm" 1.0 1.0 0.0 null null)))

(event `TakeDamage`
  (params (Damage :type "Float (double-precision)"))
  (bind _returnvalue (`GameplayStatics.GetPlayerController` 0))
  (bind _health (`self.Health`))
  (if (> _health 0.0)
    (set `self.Health` (- _health Damage))
    (bind _returnvalue_2 (`|CreateWidget` "/Game/Characters/Player/WB_Damage.WB_Damage_C"))
    (`UserWidget.AddToViewport` _returnvalue_2 20)
    (`/Game/Characters/Player/WB_Damage.ShowDamage` _returnvalue_2)
    (`KismetSystemLibrary.Delay` 2.0)
    (`UserWidget.RemoveExtension` _returnvalue_2 null)
    (else
      (bind _returnvalue_3 (`|CreateWidget` "/Game/_UI/WBP_Restart.WBP_Restart_C"))
      (`UserWidget.AddToViewport` _returnvalue_3 0)
      (`WidgetBlueprintLibrary.SetInputMode_UIOnlyEx` _returnvalue null)
      ; Comment
      (set `PlayerController.bShowMouseCursor` true _returnvalue))))

(fn `Interact`)

(fn `Shoot_Primary`
  (bind _as_bp_smart_gun (`self.As BP Smart Gun`))
  (bind _as_bp_smart_gun_2 (`self.As BP Smart Gun`))
  (bind _fp_camera (`self.FP_Camera`))
  (bind _as_bp_smart_gun_3 (`self.As BP Smart Gun`))
  (bind _fp_camera_2 (`self.FP_Camera`))
  (bind _fp_camera_3 (`self.FP_Camera`))
  (bind _asbp_smart_gun (cast `/Game/BluePrints/BP_SmartGun` (`self.CurrentWeapon`)))
  (set `self.As BP Smart Gun` _asbp_smart_gun)
  (switch `int` (`self.WeaponModeControl`)
    (:`1`
      (if (> (`/Game/BluePrints/BP_SmartGun.currentEnergy` (`self.As BP Smart Gun`)) 4.0)
        (bind _outhit (`KismetSystemLibrary.LineTraceSingle` (`SceneComponent.K2_GetComponentLocation` (`self.FP_Camera`)) (+ (`SceneComponent.K2_GetComponentLocation` _fp_camera_3) (* (`SceneComponent.GetForwardVector` _fp_camera_3) 5000)) "TraceTypeQuery1"))
        (bind (_bblockinghit _binitialoverlap _time _distance _location) (`GameplayStatics.BreakHitResult` _outhit))
        (`KismetSystemLibrary.DrawDebugSphere` _location 100.0 12 (struct :`R` 1.0 :`B` 0.960515 :`A` 1.0))
        (`GameplayStatics.PlaySound2D` "/Game/SFX/freesound_community-shoot-1-81135.freesound_community-shoot-1-81135" 1.0 1.0 0.0 null null)
        (set `/Game/BluePrints/BP_SmartGun.currentEnergy` (- (`/Game/BluePrints/BP_SmartGun.currentEnergy` _as_bp_smart_gun) 5.0) _as_bp_smart_gun)
        (`/Game/BluePrints/BP_SmartGun.OnSoundEmitted` _as_bp_smart_gun _location)
        (bind _outactors (`GameplayStatics.GetAllActorsWithInterface` "/Game/BluePrints/BPI_Hearable.BPI_Hearable_C"))
        (for _array_element _outactors
          (message `/Game/BluePrints/BPI_Hearable.HearSound` _array_element _location)
          (`/Game/_UI/WBP_Crosshair.SetEnergy` (`self.Widget`) (`KismetStringLibrary.Conv_DoubleToString` (`/Game/BluePrints/BP_SmartGun.currentEnergy` (`self.As BP Smart Gun`))))
          (`GameplayStatics.SpawnEmitterAtLocation` "/Game/StarterContent/Particles/P_Explosion.P_Explosion" (`SceneComponent.GetSocketLocation` (`/Game/BluePrints/BP_SmartGun.GunMesh` (`self.As BP Smart Gun`)) "FirePoint") (struct) (0.2 0.2 0.2)))))
    (:`2`
      (if (> (`/Game/BluePrints/BP_SmartGun.currentEnergy` (`self.As BP Smart Gun`)) 14.0)
        (set `/Game/BluePrints/BP_SmartGun.currentEnergy` (- (`/Game/BluePrints/BP_SmartGun.currentEnergy` _as_bp_smart_gun_3) 15.0) _as_bp_smart_gun_3)
        (bind _outhit_2 (`KismetSystemLibrary.LineTraceSingle` (`SceneComponent.K2_GetComponentLocation` (`self.FP_Camera`)) (+ (`SceneComponent.K2_GetComponentLocation` _fp_camera_2) (* (`SceneComponent.GetForwardVector` _fp_camera_2) 5000)) "TraceTypeQuery1"))
        (bind (_bblockinghit_2 _binitialoverlap_2 _time_2 _distance_2 _location_2 _impactpoint _normal _impactnormal _physmat _hitactor) (`GameplayStatics.BreakHitResult` _outhit_2))
        (`KismetSystemLibrary.DrawDebugSphere` _location_2)
        (`GameplayStatics.PlaySound2D` "/Game/SFX/freesound_community-shoot-5-102360.freesound_community-shoot-5-102360" 1.0 1.0 0.0 null null)
        (set `self.Shooting` true)
        (message `/Game/BluePrints/BPI_Activatable.Activate` _hitactor)
        (`/Game/_UI/WBP_Crosshair.SetEnergy` (`self.Widget`) (`KismetStringLibrary.Conv_DoubleToString` (`/Game/BluePrints/BP_SmartGun.currentEnergy` (`self.As BP Smart Gun`))))
        (`GameplayStatics.SpawnEmitterAtLocation` "/Game/StarterContent/Particles/P_Explosion.P_Explosion" (`SceneComponent.GetSocketLocation` (`/Game/BluePrints/BP_SmartGun.GunMesh` (`self.As BP Smart Gun`)) "FirePoint") (struct) (0.2 0.2 0.2))))
    (:`3`
      (if (> (`/Game/BluePrints/BP_SmartGun.currentEnergy` (`self.As BP Smart Gun`)) 24.0)
        (bind _outhit_3 (`KismetSystemLibrary.LineTraceSingle` (`SceneComponent.K2_GetComponentLocation` (`self.FP_Camera`)) (+ (`SceneComponent.K2_GetComponentLocation` _fp_camera) (* (`SceneComponent.GetForwardVector` _fp_camera) 5000)) "TraceTypeQuery1"))
        (bind (_bblockinghit_3 _binitialoverlap_3 _time_3 _distance_3 _location_3 _impactpoint_2 _normal_2 _impactnormal_2 _physmat_2 _hitactor_2) (`GameplayStatics.BreakHitResult` _outhit_3))
        (`KismetSystemLibrary.DrawDebugSphere` _location_3)
        (`GameplayStatics.PlaySound2D` "/Game/SFX/freesound_community-shoot-6-81136.freesound_community-shoot-6-81136" 1.0 1.0 0.0 null null)
        (set `/Game/BluePrints/BP_SmartGun.currentEnergy` (- (`/Game/BluePrints/BP_SmartGun.currentEnergy` _as_bp_smart_gun_2) 25.0) _as_bp_smart_gun_2)
        (set `self.Shooting` true)
        (message `/Game/BluePrints/BPI_GetDamage.Damage` _hitactor_2)
        (`/Game/_UI/WBP_Crosshair.SetEnergy` (`self.Widget`) (`KismetStringLibrary.Conv_DoubleToString` (`/Game/BluePrints/BP_SmartGun.currentEnergy` (`self.As BP Smart Gun`))))
        (`GameplayStatics.SpawnEmitterAtLocation` "/Game/StarterContent/Particles/P_Explosion.P_Explosion" (`SceneComponent.GetSocketLocation` (`/Game/BluePrints/BP_SmartGun.GunMesh` (`self.As BP Smart Gun`)) "FirePoint") (struct) (0.2 0.2 0.2))))))

(fn `Shoot_Secondary`
  (bind _returnvalue (`self.K2_GetActorLocation`))
  (bind _returnvalue_2 (`self.K2_GetActorLocation`))
  (bind _as_bp_smart_gun (`self.As BP Smart Gun`))
  (bind _fp_camera (`self.FP_Camera`))
  (bind _as_bp_smart_gun_2 (`self.As BP Smart Gun`))
  (bind _as_bp_smart_gun_3 (`self.As BP Smart Gun`))
  (bind _asbp_smart_gun (cast `/Game/BluePrints/BP_SmartGun` (`self.CurrentWeapon`)))
  (set `self.As BP Smart Gun` _asbp_smart_gun)
  (switch `int` (`self.WeaponModeControl`)
    (:`1`
      (if (> (`/Game/BluePrints/BP_SmartGun.currentEnergy` (`self.As BP Smart Gun`)) 14.0)
        (`KismetSystemLibrary.DrawDebugSphere` _returnvalue)
        (`GameplayStatics.PlaySound2D` "/Game/SFX/freesound_community-shoot-1-81135.freesound_community-shoot-1-81135" 1.0 1.0 0.0 null null)
        (set `/Game/BluePrints/BP_SmartGun.currentEnergy` (- (`/Game/BluePrints/BP_SmartGun.currentEnergy` _as_bp_smart_gun_2) 5.0) _as_bp_smart_gun_2)
        (set `self.Shooting` true)
        (`/Game/BluePrints/BP_SmartGun.OnSoundEmitted` _as_bp_smart_gun_2 _returnvalue)
        (bind _outactors (`GameplayStatics.GetAllActorsWithInterface` "/Game/BluePrints/BPI_Hearable.BPI_Hearable_C"))
        (for _array_element _outactors
          (message `/Game/BluePrints/BPI_Hearable.HearSound` _array_element _returnvalue)
          (`/Game/_UI/WBP_Crosshair.SetEnergy` (`self.Widget`) (`KismetStringLibrary.Conv_DoubleToString` (`/Game/BluePrints/BP_SmartGun.currentEnergy` (`self.As BP Smart Gun`))))
          (`GameplayStatics.SpawnEmitterAtLocation` "/Game/StarterContent/Particles/P_Explosion.P_Explosion" (`SceneComponent.GetSocketLocation` (`/Game/BluePrints/BP_SmartGun.GunMesh` (`self.As BP Smart Gun`)) "FirePoint") (struct) (0.2 0.2 0.2)))))
    (:`2`
      (if (> (`/Game/BluePrints/BP_SmartGun.currentEnergy` _as_bp_smart_gun_3) 14.0)
        (set `/Game/BluePrints/BP_SmartGun.currentEnergy` (- (`/Game/BluePrints/BP_SmartGun.currentEnergy` _as_bp_smart_gun_3) 15.0) _as_bp_smart_gun_3)
        (bind _outhits (`KismetSystemLibrary.SphereTraceMulti` _returnvalue_2 _returnvalue_2 300.0 "TraceTypeQuery1"))
        (for _array_element_2 _outhits
          (bind (_bblockinghit _binitialoverlap _time _distance _location _impactpoint _normal _impactnormal _physmat _hitactor) (`GameplayStatics.BreakHitResult` _array_element_2))
          (`KismetSystemLibrary.DrawDebugSphere` _location 300.0 12 (struct :`G` 0.905536 :`B` 1.0 :`A` 1.0))
          (`GameplayStatics.PlaySound2D` "/Game/SFX/freesound_community-shoot-5-102360.freesound_community-shoot-5-102360" 1.0 1.0 0.0 null null)
          (if (`KismetSystemLibrary.DoesImplementInterface` _hitactor "/Game/BluePrints/BPI_Activatable.BPI_Activatable_C")
            (message `/Game/BluePrints/BPI_Activatable.Activate` _hitactor)
            (`/Game/_UI/WBP_Crosshair.SetEnergy` (`self.Widget`) (`KismetStringLibrary.Conv_DoubleToString` (`/Game/BluePrints/BP_SmartGun.currentEnergy` (`self.As BP Smart Gun`))))
            (`GameplayStatics.SpawnEmitterAtLocation` "/Game/StarterContent/Particles/P_Explosion.P_Explosion" (`SceneComponent.GetSocketLocation` (`/Game/BluePrints/BP_SmartGun.GunMesh` (`self.As BP Smart Gun`)) "FirePoint") (struct) (0.2 0.2 0.2))))))
    (:`3`
      (if (> (`/Game/BluePrints/BP_SmartGun.currentEnergy` (`self.As BP Smart Gun`)) 24.0)
        (bind _outhit (`KismetSystemLibrary.LineTraceSingle` (`SceneComponent.K2_GetComponentLocation` (`self.FP_Camera`)) (+ (`SceneComponent.K2_GetComponentLocation` _fp_camera) (* (`SceneComponent.GetForwardVector` _fp_camera) 5000)) "TraceTypeQuery1"))
        (bind (_bblockinghit_2 _binitialoverlap_2 _time_2 _distance_2 _location_2 _impactpoint_2 _normal_2 _impactnormal_2 _physmat_2 _hitactor_2) (`GameplayStatics.BreakHitResult` _outhit))
        (`KismetSystemLibrary.DrawDebugSphere` _location_2)
        (`GameplayStatics.PlaySound2D` "/Game/SFX/freesound_community-shoot-6-81136.freesound_community-shoot-6-81136" 1.0 1.0 0.0 null null)
        (set `/Game/BluePrints/BP_SmartGun.currentEnergy` (- (`/Game/BluePrints/BP_SmartGun.currentEnergy` _as_bp_smart_gun) 25.0) _as_bp_smart_gun)
        (message `/Game/BluePrints/BPI_GetDamage.Explote` _hitactor_2)
        (`/Game/_UI/WBP_Crosshair.SetEnergy` (`self.Widget`) (`KismetStringLibrary.Conv_DoubleToString` (`/Game/BluePrints/BP_SmartGun.currentEnergy` (`self.As BP Smart Gun`))))
        (`GameplayStatics.SpawnEmitterAtLocation` "/Game/StarterContent/Particles/P_Explosion.P_Explosion" (`SceneComponent.GetSocketLocation` (`/Game/BluePrints/BP_SmartGun.GunMesh` (`self.As BP Smart Gun`)) "FirePoint") (struct) (0.2 0.2 0.2))))))

(fn `UserConstructionScript`)