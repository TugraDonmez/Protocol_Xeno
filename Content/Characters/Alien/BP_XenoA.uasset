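; BP_XenoA is an alien enemy that hunts the player and restarts the current level when it gets close while not stunned.
; Tick checks player distance for kills and timed growls, and reads the CanSeePlayer blackboard key to raise move speed and trigger chase sound and music.
; Damage stuns it temporarily, and HearSound records a noise location, both writing blackboard keys.
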(event `self.ReceiveBeginPlay`
  (bind _returnvalue (`GameplayStatics.GetCurrentLevelName` true))
  (set `self.Level` _returnvalue))

(event `self.ReceiveTick`
  (params (DeltaSeconds :type "Float (single-precision)"))
  (`|ExecutionSequence`
    (:`then_0`
      (if (<= (`self.GetDistanceTo` (`GameplayStatics.GetPlayerPawn` 0)) 120.0)
        (`self.KillPlayer`)))
    (:`then_1`
      (if (`BlackboardComponent.GetValueAsBool` (`AIBlueprintHelperLibrary.GetBlackboard` null) (`KismetStringLibrary.Conv_StringToName` "CanSeePlayer"))
        (set `CharacterMovementComponent.MaxWalkSpeed` 380.0 (`self.CharacterMovement`))
        (if (not (`self.MusicPlayed`))
          (`GameplayStatics.PlaySoundAtLocation` "/Game/SFX/MonsterSee.MonsterSee" (0.0 0.0 0.0) (struct) 0.6 1.0 0.0 null null null null)
          (`GameplayStatics.PlaySound2D` "/Game/SFX/Escape_Music.Escape_Music" 1.0 1.0 0.0 null null)
          (set `self.MusicPlayed` true)
          (`KismetSystemLibrary.Delay` 6.0)
          (set `self.MusicPlayed` false))
        (else
          (set `CharacterMovementComponent.MaxWalkSpeed` 150.0 (`self.CharacterMovement`)))))
    (:`then_2`
      (if (<= (`self.GetDistanceTo` (`GameplayStatics.GetPlayerPawn` 0)) 1500.0)
        (`KismetSystemLibrary.Delay` 5.0)
        (`GameplayStatics.PlaySoundAtLocation` "/Game/SFX/MonsterGrow.MonsterGrow" (`self.K2_GetActorLocation`) (struct) 1.0 1.0 0.0 null null null null)))))

(event `KillPlayer`
  (if (not (`self.IsStunned`))
    (`GameplayStatics.PlaySound2D` "/Game/StarterContent/Audio/Explosion01.Explosion01" 1.0 1.0 0.0 null null)
    (`GameplayStatics.OpenLevel` (`KismetStringLibrary.Conv_StringToName` (`self.Level`)))))

(event `/Game/BluePrints/BPI_GetDamage.Damage`
  (`BlackboardComponent.SetValueAsBool` (`AIBlueprintHelperLibrary.GetBlackboard` null) (`KismetStringLibrary.Conv_StringToName` "IsStunned") true)
  (set `self.IsStunned` true)
  (`KismetSystemLibrary.Delay` 5.0)
  (`BlackboardComponent.SetValueAsBool` (`AIBlueprintHelperLibrary.GetBlackboard` null) (`KismetStringLibrary.Conv_StringToName` "IsStunned") false)
  (set `self.IsStunned` false))

(event `/Game/BluePrints/BPI_Hearable.HearSound`
  (params (TargetLocation :type "Vector Structure"))
  (bind _returnvalue (`AIBlueprintHelperLibrary.GetBlackboard` null))
  (`BlackboardComponent.SetValueAsBool` _returnvalue (`KismetStringLibrary.Conv_StringToName` "Hear") true)
  (`BlackboardComponent.SetValueAsVector` _returnvalue (`KismetStringLibrary.Conv_StringToName` "LastKnownLocation") TargetLocation))

(fn `UserConstructionScript`)