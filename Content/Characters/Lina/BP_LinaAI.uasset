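; Lina's ally character, which moves to target actors or heard sound locations through its AIC_AllyAI controller.
; GoToLocation flags waiting and calls OnArrived immediately after issuing the move, without awaiting completion.
; While waiting, a player overlapping the Wait component triggers GoToLocation again, though this call and StartPatrol's pass no target.
; Capsule overlaps automatically open closed BP_DoorB and BP_Door_250cm doors.
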(event `self.ReceiveTick`
  (params (DeltaSeconds :type "Float (single-precision)")))

(event `GoToLocation`
  (params (TargetActor :type "Actor Object Reference"))
  (set `self.IsMoving` true)
  (bind _asaic_ally_ai (cast `/Game/BluePrints/AIC_AllyAI` (`self.GetController`)))
  (`AIController.MoveToActor` _asaic_ally_ai TargetActor 50.0 true true true null true)
  (set `self.IsMoving` false)
  (`self.OnArrived`))

(event `OnArrived`
  (set `self.IsWaiting` true)
  (`KismetSystemLibrary.PrintString` "hedefe varıldı"))

(event `/Game/BluePrints/BPI_Hearable.HearSound`
  (params (TargetLocation :type "Vector Structure"))
  (bind _asaic_ally_ai (cast `/Game/BluePrints/AIC_AllyAI` (`self.GetController`)))
  (`AIController.MoveToLocation` _asaic_ally_ai TargetLocation 50.0 true true false true null true))

(event `StartPatrol`
  (set `self.IsWaiting` false)
  (`self.GoToLocation` null))

(event `self.CapsuleComponent.OnComponentBeginOverlap`
  (params (OverlappedComponent :type "PrimitiveComponent Object Reference") (OtherActor :type "Actor Object Reference") (OtherComp :type "PrimitiveComponent Object Reference") (OtherBodyIndex :type Integer) (bFromSweep :type Boolean) (SweepResult :type "HitResult Structure (by ref)"))
  (bind _asbp_door_b (cast `/Game/QA_Office/Blueprints/BP_DoorB` OtherActor)
    (:`then`
      (if (`/Game/QA_Office/Blueprints/BP_DoorB.DoorClosed` _asbp_door_b)
        (`/Game/QA_Office/Blueprints/BP_DoorB.DoorOpening` _asbp_door_b)))
    (:`CastFailed`
      (bind _asbp_door_250cm (cast `/Game/QA_Office/Blueprints/BP_Door_250cm` OtherActor))
      (if (`/Game/QA_Office/Blueprints/BP_Door_250cm.DoorClosed` _asbp_door_250cm)
        (`/Game/QA_Office/Blueprints/BP_Door_250cm.DoorOpening` _asbp_door_250cm)))))

(event `self.Wait.OnComponentBeginOverlap`
  (params (OverlappedComponent :type "PrimitiveComponent Object Reference") (OtherActor :type "Actor Object Reference") (OtherComp :type "PrimitiveComponent Object Reference") (OtherBodyIndex :type Integer) (bFromSweep :type Boolean) (SweepResult :type "HitResult Structure (by ref)"))
  (cast `/Game/Characters/Player/BP_PlayerCharacterFPS` OtherActor)
  (if (`self.IsWaiting`)
    (`self.GoToLocation` null)
    (set `self.IsWaiting` false)))

(fn `UserConstructionScript`)