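; Ally AI character Lina, who travels to placed target actors, waits for the player and opens doors.
; Events write movement, cinematic and waiting flags to the AIC_AllyAI blackboard; play begins in cinematic mode.
; Ending the cinematic sets the next target location, then fixes the target index at 1.
; Tick toggles waiting by player distance, and capsule overlap opens closed BP_DoorB or BP_Door_250cm doors.
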(event `SetNextTarget`
  (bind _asaic_ally_ai (cast `/Game/BluePrints/AIC_AllyAI` (`self.GetController`))
    (:`then`
      (bind _returnvalue (`AIBlueprintHelperLibrary.GetBlackboard` _asaic_ally_ai))
      (`BlackboardComponent.SetValueAsVector` _returnvalue (`KismetStringLibrary.Conv_StringToName` "TargetLocation") (`self.K2_GetActorLocation` (`|GetArrayItem` (`self.Target_1`) (`self.GoIndex`))))
      (`BlackboardComponent.SetValueAsBool` _returnvalue (`KismetStringLibrary.Conv_StringToName` "CanMove") true)
      (`BlackboardComponent.SetValueAsBool` _returnvalue (`KismetStringLibrary.Conv_StringToName` "IsWaiting") false)
      (set `self.GoIndex` 1))
    (:`CastFailed`
      (`KismetSystemLibrary.PrintString` "Fail"))))

(event `self.ReceiveBeginPlay`
  (`self.StartCinematic`))

(event `self.ReceiveTick`
  (params (DeltaSeconds :type "Float (single-precision)"))
  (if (> (`self.GetDistanceTo` (`GameplayStatics.GetPlayerPawn` 0)) 400.0)
    (`self.StartWaiting`)
    (else
      (`self.EndWaiting`))))

(event `StartCinematic`
  (bind _asaic_ally_ai (cast `/Game/BluePrints/AIC_AllyAI` (`self.GetController`)))
  (bind _returnvalue (`AIBlueprintHelperLibrary.GetBlackboard` _asaic_ally_ai))
  (`BlackboardComponent.SetValueAsBool` _returnvalue (`KismetStringLibrary.Conv_StringToName` "CanMove") false)
  (`BlackboardComponent.SetValueAsBool` _returnvalue (`KismetStringLibrary.Conv_StringToName` "IsCinematic") true))

(event `EndCinematic`
  (bind _asaic_ally_ai (cast `/Game/BluePrints/AIC_AllyAI` (`self.GetController`)))
  (`BlackboardComponent.SetValueAsBool` (`AIBlueprintHelperLibrary.GetBlackboard` _asaic_ally_ai) (`KismetStringLibrary.Conv_StringToName` "IsCinematic") false)
  (`self.SetNextTarget`))

(event `StartWaiting`
  (bind _asaic_ally_ai (cast `/Game/BluePrints/AIC_AllyAI` (`self.GetController`)))
  (`BlackboardComponent.SetValueAsBool` (`AIBlueprintHelperLibrary.GetBlackboard` _asaic_ally_ai) (`KismetStringLibrary.Conv_StringToName` "IsWaiting") true))

(event `self.CapsuleComponent.OnComponentBeginOverlap`
  (params (OverlappedComponent :type "PrimitiveComponent Object Reference") (OtherActor :type "Actor Object Reference") (OtherComp :type "PrimitiveComponent Object Reference") (OtherBodyIndex :type Integer) (bFromSweep :type Boolean) (SweepResult :type "HitResult Structure (by ref)"))
  (bind _asbp_door_b (cast `/Game/QA_Office/Blueprints/BP_DoorB` OtherActor)
    (:`then`
      (if (`/Game/QA_Office/Blueprints/BP_DoorB.DoorClosed` _asbp_door_b)
        (`/Game/QA_Office/Blueprints/BP_DoorB.DoorOpening` _asbp_door_b)))
    (:`CastFailed`
      (bind _asbp_door_250cm (cast `/Game/QA_Office/Blueprints/BP_Door_250cm` OtherActor))
      (if (`/Game/QA_Office/Blueprints/BP_Door_250cm.DoorClosed` _asbp_door_250cm)
        (`/Game/QA_Office/Blueprints/BP_Door_250cm.DoorOpening` _asbp_door_250cm)))))

(event `EndWaiting`
  (bind _asaic_ally_ai (cast `/Game/BluePrints/AIC_AllyAI` (`self.GetController`)))
  (`BlackboardComponent.SetValueAsBool` (`AIBlueprintHelperLibrary.GetBlackboard` _asaic_ally_ai) (`KismetStringLibrary.Conv_StringToName` "IsWaiting") false))

(fn `UserConstructionScript`)